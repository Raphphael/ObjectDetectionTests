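; BP_ObjectLabel is a placeable AR toolkit actor that shows a text label which turns to face the player's camera.
; On BeginPlay it caches the camera from BP_ARPawn and applies its Text variable to the TextRender component.
; Each Tick it smoothly rotates the TextRender toward that camera using a look-at rotation and RInterpTo.
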(event `self.ReceiveBeginPlay`
  (bind _asbp_arpawn (cast `/Game/AR_toolkit/Blueprints/GameFramework/BP_ARPawn` (`GameplayStatics.GetPlayerPawn` 0)))
  (set `self.pawn camera` (`/Game/AR_toolkit/Blueprints/GameFramework/BP_ARPawn.Camera` _asbp_arpawn))
  (`TextRenderComponent.K2_SetText` (`self.TextRender`) (`self.text`)))

(event `self.ReceiveTick`
  (params (DeltaSeconds :type "Float (single-precision)"))
  (bind _textrender (`self.TextRender`))
  (`SceneComponent.K2_SetWorldRotation` _textrender (`KismetMathLibrary.RInterpTo` (`SceneComponent.K2_GetComponentRotation` _textrender) (`KismetMathLibrary.FindLookAtRotation` (`SceneComponent.K2_GetComponentLocation` (`self.TextRender`)) (`SceneComponent.K2_GetComponentLocation` (`self.pawn camera`))) DeltaSeconds 4.0) false false))

(fn `UserConstructionScript`)