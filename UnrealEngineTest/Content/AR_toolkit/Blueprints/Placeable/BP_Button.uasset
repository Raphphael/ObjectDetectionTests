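; BP_Button is a placeable AR actor that shows a numbered button widget as a world-space label facing the player.
; On BeginPlay it passes its number, unlock state, model reference and text number to BP_Widget_Button, then caches the BP_ARPawn camera.
; Tick smoothly rotates the widget toward that camera and scales it by distance over viewport size, keeping its apparent size uniform.
; UpdateWidgetbuttons refreshes the widget's button styles.
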(event `self.ReceiveBeginPlay`
  ;[0 0 0] set up variables
  (bind _asbp_widget_button (cast `/Game/AR_toolkit/Blueprints/UI/Widgets/BP_Widget_Button` (`WidgetComponent.GetUserWidgetObject` (`self.Widget`))))
  (bind _output_get (set `self.button widget` _asbp_widget_button))
  (set `/Game/AR_toolkit/Blueprints/UI/Widgets/BP_Widget_Button.Button number` (`KismetTextLibrary.Conv_IntToText` (`self.button number`)) _output_get)
  (set `/Game/AR_toolkit/Blueprints/UI/Widgets/BP_Widget_Button.WidgetEnabled` (`self.BP unlocked`) _output_get)
  (set `/Game/AR_toolkit/Blueprints/UI/Widgets/BP_Widget_Button.BP model ref` (`self.BP model ref`) _asbp_widget_button)
  (set `/Game/AR_toolkit/Blueprints/UI/Widgets/BP_Widget_Button.UI text number` (`self.UI text number`) _asbp_widget_button)
  (bind _asbp_arpawn (cast `/Game/AR_toolkit/Blueprints/GameFramework/BP_ARPawn` (`GameplayStatics.GetPlayerPawn` 0)))
  (set `self.pawn camera` (`/Game/AR_toolkit/Blueprints/GameFramework/BP_ARPawn.Camera` _asbp_arpawn)))

(event `Update Widget buttons`
  ;[0 0 0] Update buttons
  (bind _asbp_widget_button (cast `/Game/AR_toolkit/Blueprints/UI/Widgets/BP_Widget_Button` (`WidgetComponent.GetUserWidgetObject` (`self.Widget`))))
  (`/Game/AR_toolkit/Blueprints/UI/Widgets/BP_Widget_Button.update button styles` _asbp_widget_button))

(event `self.ReceiveTick`
  (params (DeltaSeconds :type "Float (single-precision)"))
  (bind _widget (`self.Widget`))
  ;[0 0 0] make label follow player and scale uniformly based on distance
  (bind _returnvalue (`self.Rotate towards camera` DeltaSeconds))
  (`SceneComponent.K2_SetWorldRotation` _widget _returnvalue false false)
  (`SceneComponent.SetWorldScale3D` _widget (`self.get scale relative to camera`)))

(fn `get scale relative to camera`
  (returns (ReturnValue :type "Vector Structure"))
  (bind (_x _y) (`KismetMathLibrary.BreakVector2D` (`WidgetLayoutLibrary.GetViewportSize`)))
  (return (`KismetMathLibrary.Conv_DoubleToVector` (* (/ (`KismetMathLibrary.VSize` (- (`SceneComponent.K2_GetComponentLocation` (`self.pawn camera`)) (`SceneComponent.K2_GetComponentLocation` (`self.Widget`)))) (+ _x _y)) 0.75))))

(fn `Rotate towards camera`
  (params (DeltaTime :type "Float (double-precision)"))
  (returns (ReturnValue :type "Rotator Structure"))
  (return (`KismetMathLibrary.RInterpTo` (`SceneComponent.K2_GetComponentRotation` (`self.Widget`)) (`KismetMathLibrary.FindLookAtRotation` (`SceneComponent.K2_GetComponentLocation` (`self.Widget`)) (`SceneComponent.K2_GetComponentLocation` (`self.pawn camera`))) DeltaTime 4.0)))

(fn `UserConstructionScript`
  (bind _widget (`self.Widget`))
  (bind (_x _y) (`KismetMathLibrary.BreakVector2D` (`WidgetLayoutLibrary.GetViewportSize`)))
  (if (> (+ _x _y) 2000.0)
    (`SceneComponent.SetWorldScale3D` _widget (0.02 0.02 0.02))
    (else
      (`SceneComponent.SetWorldScale3D` _widget (0.05 0.05 0.05)))))