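; Placeable AR model actor that spawns attached BP_Button actors at mesh sockets prefixed "btn", numbered by the socket's last digit.
; ButtonSelection resets all materials, then highlights the slot named after the socket.
; Resettimer shows the actor and re-arms a timer that hides it when image tracking stops.
; Tick turns and scales the percentage widget by camera position, while a passthrough material is applied to the shadow plane.
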(event `self.ReceiveBeginPlay`
  (bind _model (`self.Model`))
  (`|ExecutionSequence`
    (:`then_0`
      ;[0 0 0] set up variables
      (bind _asbp_arpawn (cast `/Game/AR_toolkit/Blueprints/GameFramework/BP_ARPawn` (`GameplayStatics.GetPlayerPawn` 0))
        (:`then`
          (set `self.pawn` _asbp_arpawn)
          (set `self.camera` (`/Game/AR_toolkit/Blueprints/GameFramework/BP_ARPawn.Camera` _asbp_arpawn)))
        (:`CastFailed`
          _))
      ;[0 0 0] if there are mulitple meshes with sockets add them to the array
      (if (`self.Single mesh`)
        ;[0 0 0] make a button for every mesh socket
        (for _array_element (`SceneComponent.GetAllSocketNames` _model) :!label _label
          (`self.add new button` _array_element _model))
        (else
          (bind _output_get (set `self.ButtonMeshes` (`|MakeArray` null null null null null null :!type "StaticMeshComponent Object Reference"))) ; create button meshes array
          (for _ _output_get
            (goto _label)))))
    (:`then_1`
      ;[0 0 0] Apply passthrough material to plane for shadow casting
      (bind _returnvalue (`AddComponent|NODE_AddPassthroughMaterialUpdateComponent-0`))
      (`PassthroughMaterialUpdateComponent.AddAffectedComponent` _returnvalue (`self.Shadow Plane Dynamic`)))))

(event `self.ReceiveTick`
  (params (DeltaSeconds :type "Float (single-precision)"))
  ;[0 0 0] update widget rotation to face camera
  (bind _returnvalue (`self.Rotate towards camera` DeltaSeconds))
  (`SceneComponent.K2_SetWorldRotation` (`self.Scale Percentage Widget`) _returnvalue false false)
  ;[0 0 0] update widget scale
  (`SceneComponent.SetWorldScale3D` (`self.Scale Percentage Widget`) (`self.Scale based on camera distance` (`self.scale multiplier`))))

(event `Reset timer`
  (`KismetSystemLibrary.K2_SetTimerDelegate` (delegate `Set model to hidden`) 0.5) ; Keep reseting timer while the image is tracked
  (`self.SetActorHiddenInGame` false) ; Show model
)

(event `Set model to hidden`
  (`self.SetActorHiddenInGame` true) ; hide model
)

(event `Button Selection`
  (params (`Button Number` :type Integer) (MaterialHighlightName :type Name))
  (bind _model (`self.Model`))
  ;[0 0 0] Highlight meshes
  (for _index (range (+ (`PrimitiveComponent.GetNumMaterials` _model) 1))
    (`PrimitiveComponent.SetMaterial` _model _index "/Game/AR_toolkit/Materials/M_PumpJack.M_PumpJack"))
  (switch `int` `Button Number`
    (:`Default`
      _)
    (:`1`
      (`KismetSystemLibrary.PrintString` "Button 1 custom event"))
    (:`2`
      (`KismetSystemLibrary.PrintString` "Button 2 custom event"))
    (:`3`
      (`KismetSystemLibrary.PrintString` "Button 3 custom event")))
  (`PrimitiveComponent.SetMaterialByName` (`self.Model`) MaterialHighlightName "/Game/AR_toolkit/Materials/M_PumpJackHighlight.M_PumpJackHighlight") ; highlight material at slot
)

(fn `add new button`
  (params (`Socket name` :type Name) (Mesh :type "SceneComponent Object Reference"))
  (bind _returnvalue (`KismetStringLibrary.Conv_NameToString` `Socket name`))
  (if (`KismetStringLibrary.StartsWith` _returnvalue "btn")
    (bind _returnvalue_2 (`|SpawnActorFromClass` "/Game/AR_toolkit/Blueprints/Placeable/BP_Button.BP_Button_C" (`SceneComponent.GetSocketTransform` Mesh `Socket name` "RTS_World") "Undefined" "OverrideRootScale" null (`KismetStringLibrary.Conv_StringToInt` (`KismetStringLibrary.Right` _returnvalue 1)) (`self.all buttons unlocked`) `Socket name` self (`self.UI text number`) null))
    (`self.K2_AttachToActor` _returnvalue_2 self "None" "KeepWorld" "KeepWorld" "KeepWorld" true)
    (`KismetArrayLibrary.Array_Add` (`self.buttons`) _returnvalue_2)))

(fn `Hide Shadow Plane`
  (`SceneComponent.SetHiddenInGame` (`self.Shadow Plane Dynamic`) true true))

(fn `Rotate towards camera`
  (params (DeltaTime :type "Float (double-precision)"))
  (returns (ReturnValue :type "Rotator Structure"))
  (return (`KismetMathLibrary.RInterpTo` (`SceneComponent.K2_GetComponentRotation` (`self.Scale Percentage Widget`)) (`KismetMathLibrary.FindLookAtRotation` (`SceneComponent.K2_GetComponentLocation` (`self.Scale Percentage Widget`)) (`SceneComponent.K2_GetComponentLocation` (`self.camera`))) DeltaTime 4.0)))

(fn `Scale based on camera distance`
  (params (`Scale Multiplier` :type "Float (double-precision)"))
  (returns (ReturnValue :type "Vector Structure"))
  (bind (_x _y) (`KismetMathLibrary.BreakVector2D` (`WidgetLayoutLibrary.GetViewportSize`)))
  (return (`KismetMathLibrary.Conv_DoubleToVector` (* (/ (`KismetMathLibrary.VSize` (- (`SceneComponent.K2_GetComponentLocation` (`self.camera`)) (`SceneComponent.K2_GetComponentLocation` (`self.Scale Percentage Widget`)))) (+ _x _y)) `Scale Multiplier`))))

(fn `UserConstructionScript`)