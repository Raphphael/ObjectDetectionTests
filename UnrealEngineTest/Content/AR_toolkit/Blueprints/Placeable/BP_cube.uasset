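; BP_cube is a short-lived placeable physics cube in the AR toolkit that destroys itself ten seconds after BeginPlay.
; The construction script gives its Object component a dynamic instance of M_physics_object with a random colour.
; Unconnected nodes that would push it along the BP_ARPawn camera's forward vector remain in the event graph but never run.
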(event `self.ReceiveBeginPlay`
  (`KismetSystemLibrary.Delay` 10.0)
  (`self.K2_DestroyActor`))

(fn `UserConstructionScript`
  (bind _returnvalue (`PrimitiveComponent.CreateDynamicMaterialInstance` (`self.Object`) 0 "/Game/AR_toolkit/Materials/M_physics_object.M_physics_object" "None"))
  (`MaterialInstanceDynamic.SetVectorParameterValue` _returnvalue "Colour" (`KismetMathLibrary.MakeColor` (`KismetMathLibrary.RandomFloat`) (`KismetMathLibrary.RandomFloat`) (`KismetMathLibrary.RandomFloat`))))