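; Transform gizmo actor for point cloud capture in the AR toolkit, built from X, Y and Z arrow meshes.
; Move and scale events swap every arrow's mesh and set a mode flag, with move mode active at BeginPlay.
; The construction script gives each arrow a semi-transparent dynamic material.
; A highlight event briefly flashes a given arrow to full opacity, using a gate to block re-triggering during the flash.
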(event `self.ReceiveBeginPlay`
  (`self.Move mode`))

(event `Move mode`
  (for _array_element (`|MakeArray` (`self.X+`) (`self.Y+`) (`self.Z+`) (`self.X-`) (`self.Y-`) (`self.Z-`))
    (`StaticMeshComponent.SetStaticMesh` _array_element "/Game/AR_toolkit/Meshes/ObjectScanningMeshes/SM_Arrow_move.SM_Arrow_move")
    (set `self.is Move mode` true)))

(event `scale mode`
  (for _array_element (`|MakeArray` (`self.X+`) (`self.Y+`) (`self.Z+`) (`self.X-`) (`self.Y-`) (`self.Z-`))
    (`StaticMeshComponent.SetStaticMesh` _array_element "/Game/AR_toolkit/Meshes/ObjectScanningMeshes/SM_Arrow_scale.SM_Arrow_scale")
    (set `self.is Move mode` false)))

(event `highlight`
  (params (arrow :type "ActorComponent Object Reference"))
  (if (`self.open`)
    (bind _asmesh_component (cast `MeshComponent` arrow))
    (set `self.open` false)
    (bind _returnvalue (`PrimitiveComponent.CreateDynamicMaterialInstance` _asmesh_component 0 (`PrimitiveComponent.GetMaterial` _asmesh_component 0) "None"))
    (`MaterialInstanceDynamic.SetScalarParameterValue` _returnvalue "opacity" 1.0)
    (`KismetSystemLibrary.Delay` 0.1)
    (`MaterialInstanceDynamic.SetScalarParameterValue` _returnvalue "opacity" 0.65)
    (set `self.open` true)))

(fn `UserConstructionScript`
  (for _array_element (`|MakeArray` (`self.X+`) (`self.Y+`) (`self.Z+`) (`self.X-`) (`self.Y-`) (`self.Z-`))
    (bind _returnvalue (`PrimitiveComponent.CreateDynamicMaterialInstance` _array_element 0 (`PrimitiveComponent.GetMaterial` _array_element 0) "None"))
    (`MaterialInstanceDynamic.SetScalarParameterValue` _returnvalue "opacity" 0.65)))